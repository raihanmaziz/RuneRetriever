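; Replicated cube actor that changes CurrentColor when something overlaps its box.
; BeginPlay creates a dynamic M_Solid material on the cube.
; On overlap, only the authority sets CurrentColor from GetRandomColor, and its RepNotify writes the value to the material's Base Color parameter.
; The random MakeColor node inside GetRandomColor appears unconnected, so that function may not return a random color.
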(event `self.ReceiveBeginPlay`
  (bind _returnvalue (`PrimitiveComponent.CreateDynamicMaterialInstance` (`self.Cube`) 0 "/Game/LevelPrototyping/Materials/M_Solid.M_Solid" "None"))
  (set `self.ColorMaterial` _returnvalue))

(event `self.Box.OnComponentBeginOverlap`
  (params (OverlappedComponent :type "PrimitiveComponent Object Reference") (OtherActor :type "Actor Object Reference") (OtherComp :type "PrimitiveComponent Object Reference") (OtherBodyIndex :type Integer) (bFromSweep :type Boolean) (SweepResult :type "HitResult Structure (by ref)"))
  (`/Engine/EditorBlueprintResources/ActorMacros.Switch Has Authority`
    (:`Authority`
      (set `self.CurrentColor` (`self.GetRandomColor`)))))

(fn `OnRep_CurrentColor`
  (`MaterialInstanceDynamic.SetVectorParameterValue` (`self.ColorMaterial`) "Base Color" (`self.CurrentColor`)))

(fn `UserConstructionScript`)