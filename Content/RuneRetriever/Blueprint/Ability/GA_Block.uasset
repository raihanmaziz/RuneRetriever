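; GA_Block is a Gameplay Ability that puts a RuneRetriever character into a blocking state.
; On activation it commits, applies GE_IsBlocking to the owner, and calls Blocking on the owning BP_RuneBaseCharacter.
; A WaitGameplayTagRemove task on the IsBlocking tag ends the ability when that tag is removed.
; On end it calls FinishBlocking on the character and ends the stored wait task.
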(event `self.K2_ActivateAbility`
  (`self.K2_CommitAbility`)
  (`self.BP_ApplyGameplayEffectToOwner` "/Game/RuneRetriever/Blueprint/Ability/GE_IsBlocking.GE_IsBlocking_C")
  (bind _asbp_rune_base_character (cast `/Game/ThirdPerson/Blueprints/BP_RuneBaseCharacter` (`.OwnerActor` (break `GameplayAbilityActorInfo` (`self.GetActorInfo`)))))
  (`/Game/ThirdPerson/Blueprints/BP_RuneBaseCharacter.Blocking` _asbp_rune_base_character)
  (bind _asynctaskproxy (`AbilityTask_WaitGameplayTagRemoved.WaitGameplayTagRemove` (struct :`TagName` "RuneRetriever.Character.IsBlocking") null)
    (:`then`
      (set `self.WaitForTagRemoval` _asynctaskproxy))
    (:`Removed`
      (`self.K2_EndAbility`))))

(event `self.K2_OnEndAbility`
  (params (bWasCancelled :type Boolean))
  (bind _waitfortagremoval (`self.WaitForTagRemoval`))
  (`/Game/ThirdPerson/Blueprints/BP_RuneBaseCharacter.FinishBlocking` (stale `self.K2_ActivateAbility` _asbp_rune_base_character))
  (`/Engine/EditorBlueprintResources/StandardMacros.IsValid` _waitfortagremoval
    (:`Is Valid`
      (`GameplayTask.EndTask` _waitfortagremoval))))